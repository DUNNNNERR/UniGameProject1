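; BP_WallJumpObject is a pickup that grants the top-down character the wall jump item.
; A sphere collision tracks whether the player is in range and stores a reference to the character.
; On Interact in range, it attaches to the player's mesh, offsets its static mesh, disables collision and sets HasWallJumpItem on the character.
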(event `self.SphereCollision.OnComponentBeginOverlap`
  (params (OverlappedComponent :type "PrimitiveComponent Object Reference") (OtherActor :type "Actor Object Reference") (OtherComp :type "PrimitiveComponent Object Reference") (OtherBodyIndex :type Integer) (bFromSweep :type Boolean) (SweepResult :type "HitResult Structure (by ref)"))
  ; Player in/out of range to interact
  (bind _asbp_top_down_character (cast `/Game/MainFolder/Blueprints/BP_TopDownCharacter` OtherActor))
  (set `self.PlayerRef` _asbp_top_down_character)
  (set `self.PlayerInRange` true))

(event `self.SphereCollision.OnComponentEndOverlap`
  (params (OverlappedComponent :type "PrimitiveComponent Object Reference") (OtherActor :type "Actor Object Reference") (OtherComp :type "PrimitiveComponent Object Reference") (OtherBodyIndex :type Integer))
  ; Player in/out of range to interact
  (cast `/Game/MainFolder/Blueprints/BP_TopDownCharacter` OtherActor)
  (set `self.PlayerInRange` false))

(event `/Game/MainFolder/Blueprints/BI_Interact.Interact`
  ; Interact and attach to Player logic
  (if (`self.PlayerInRange`)
    (`self.K2_AttachToComponent` (`Character.Mesh` (`self.PlayerRef`)) "None" "SnapToTarget" "SnapToTarget" "KeepWorld")
    (`SceneComponent.K2_SetRelativeLocation` (`self.StaticMesh`) (-50.0 0.0 200.0) false false)
    (`self.SetActorEnableCollision` false)
    (set `/Game/MainFolder/Blueprints/BP_TopDownCharacter.HasWallJumpItem` true (`self.PlayerRef`))
    (`PrimitiveComponent.SetCollisionEnabled` (`self.SphereCollision`) "NoCollision")))

(fn `UserConstructionScript`)