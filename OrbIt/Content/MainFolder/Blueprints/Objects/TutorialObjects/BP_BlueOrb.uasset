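; BP_BlueOrb is a tutorial object that shows an on-screen blue orb prompt when the player is near.
; On BeginPlay it creates a WBP_BlueOrb widget once and stores it for reuse.
; Its BoxCollision overlap events add that widget to the viewport when the player character enters and remove it when the player leaves.
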(event `self.ReceiveBeginPlay`
  (bind _returnvalue (`|CreateWidget` "/Game/MainFolder/Blueprints/HUDs/TutorialHUDs/WBP_BlueOrb.WBP_BlueOrb_C"))
  (set `self.BlueOrbPrompt` _returnvalue))

(event `self.BoxCollision.OnComponentBeginOverlap`
  (params (OverlappedComponent :type "PrimitiveComponent Object Reference") (OtherActor :type "Actor Object Reference") (OtherComp :type "PrimitiveComponent Object Reference") (OtherBodyIndex :type Integer) (bFromSweep :type Boolean) (SweepResult :type "HitResult Structure (by ref)"))
  (if (== OtherActor (`GameplayStatics.GetPlayerCharacter` 0))
    (`UserWidget.AddToViewport` (`self.BlueOrbPrompt`) 0)))

(event `self.BoxCollision.OnComponentEndOverlap`
  (params (OverlappedComponent :type "PrimitiveComponent Object Reference") (OtherActor :type "Actor Object Reference") (OtherComp :type "PrimitiveComponent Object Reference") (OtherBodyIndex :type Integer))
  (if (== (`GameplayStatics.GetPlayerCharacter` 0) OtherActor)
    (`Widget.RemoveFromParent` (`self.BlueOrbPrompt`))))

(fn `UserConstructionScript`)